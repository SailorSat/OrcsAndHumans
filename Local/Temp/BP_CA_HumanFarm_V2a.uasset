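; Human farm building Blueprint that reskins its static mesh to match a selected regional theme, such as Westfall, Duskwood or Stratholme.
; The construction script switches on FactionTemplate and picks the matching slot-to-material map for that theme.
; It passes that map and the mesh component to BatchUpdateMaterials, so the variant is applied at construction rather than through runtime event logic.
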(fn ConstructionScript
  (bind _staticmeshcomponent (Variables|Debug|GetStaticMeshComponent))
  (switch Utilities|FlowControl|Switch|SwitchonE_HumanFaction (Variables|Default|GetFactionTemplate)
    (:NewEnumerator1
      (CallFunction|BatchUpdateMaterials _staticmeshcomponent (LocalVariables|GetMapWestfall)))
    (:NewEnumerator2
      (CallFunction|BatchUpdateMaterials _staticmeshcomponent (LocalVariables|GetMapDuskwood)))
    (:NewEnumerator3
      (CallFunction|BatchUpdateMaterials _staticmeshcomponent (LocalVariables|GetMapRedridge)))
    (:NewEnumerator4
      (CallFunction|BatchUpdateMaterials _staticmeshcomponent (LocalVariables|GetMapKarazhan)))
    (:NewEnumerator10
      (CallFunction|BatchUpdateMaterials _staticmeshcomponent (LocalVariables|GetMapStratholme)))
    (:NewEnumerator11
      (CallFunction|BatchUpdateMaterials _staticmeshcomponent (LocalVariables|GetMapHearthglen)))))