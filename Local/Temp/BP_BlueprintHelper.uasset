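; Building helper actor that moves to BuildingPosition on BeginPlay and spawns static meshes described by its Script string.
; Each semicolon-separated entry gives a mesh path and transform, added as a world-space instance.
; A map keeps one Instanced Static Mesh component per path, loading the asset on first use.
; When not on the server, it prints each mesh path and its instances' transforms converted against BuildingPosition.
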(event EventBeginPlay
  (bind _buildingposition (Variables|Default|GetBuildingPosition))
  (Transformation|SetActorLocationAndRotation (.location _buildingposition) (.rotation _buildingposition))
  (bind _output_get (Variables|Default|SetLineArray (Utilities|String|ParseIntoArray (Variables|Default|GetScript) ";")))
  (for _array_element _output_get
    (bind _output_get_2 (Variables|Default|SetLine _array_element))
    (bind _output_get_3 (Variables|Default|SetParamArray (Utilities|String|ParseIntoArray _output_get_2 " ")))
    (Variables|Default|SetMeshName (Utilities|Array|Get(acopy) _output_get_3))
    (Variables|Default|SetMeshTransform (Math|Transform|MakeTransform (Math|Vector|MakeVector (Math|Conversions|ToFloat(Integer) (Utilities|Array|Get(acopy) _output_get_3 1)) (Math|Conversions|ToFloat(Integer) (Utilities|Array|Get(acopy) _output_get_3 2)) (Math|Conversions|ToFloat(Integer) (Utilities|Array|Get(acopy) _output_get_3 3))) (Math|Rotator|MakeRotator (Math|Conversions|ToFloat(Integer) (Utilities|Array|Get(acopy) _output_get_3 4)) (Math|Conversions|ToFloat(Integer) (Utilities|Array|Get(acopy) _output_get_3 5)) (Math|Conversions|ToFloat(Integer) (Utilities|Array|Get(acopy) _output_get_3 6))) (Math|Vector|MakeVector (Math|Conversions|ToFloat(Integer) (Utilities|Array|Get(acopy) _output_get_3 7)) (Math|Conversions|ToFloat(Integer) (Utilities|Array|Get(acopy) _output_get_3 8)) (Math|Conversions|ToFloat(Integer) (Utilities|Array|Get(acopy) _output_get_3 9)))))
    (if (.ReturnValue (Utilities|Map|Find (Variables|Default|GetInstancedStaticMeshMap) (Variables|Default|GetMeshName)))
      (bind _output_get_4 (Variables|Default|SetInstancedStaticMesh (.Value (Utilities|Map|Find (Variables|Default|GetInstancedStaticMeshMap) (Variables|Default|GetMeshName)))))
      (else
        (bind _returnvalue (Class|FuncomGenericLibrary|LoadAssetfromPath (Variables|Default|GetMeshName)))
        (bind _asstatic_mesh (Utilities|Casting|CastToStaticMesh _returnvalue))
        (Variables|Default|SetStaticMesh _asstatic_mesh)
        (bind _returnvalue_2 (AddComponent|AddInstancedStaticMeshComponent true))
        (bind _output_get_5 (Variables|Default|SetInstancedStaticMesh _returnvalue_2))
        (Utilities|Map|Add (Variables|Default|GetInstancedStaticMeshMap) (Variables|Default|GetMeshName) _output_get_5)
        (Components|StaticMesh|SetStaticMesh _output_get_5 (Variables|Default|GetStaticMesh))))
    (Class|InstancedStaticMeshComponent|AddInstanceWorldSpace _output_get_4 (Variables|Default|GetMeshTransform)))
  (if (not (Networking|IsServer))
    (bind _values (Utilities|Map|Values (Variables|Default|GetInstancedStaticMeshMap)))
    (bind _output_get_6 (Variables|Default|SetInstancedStacisMeshArray _values))
    (for _array_element_2 _output_get_6
      (bind _output_get_7 (Variables|Default|SetInstancedStaticMesh _array_element_2))
      (Development|PrintString (Class|KismetSystemLibrary|GetPathName (Variables|/Script/Engine.StaticMeshComponent|GetStaticMesh _output_get_7)))
      (bind _output_get_8 (Variables|Default|SetInstanceCount (- (Components|InstancedStaticMesh|GetInstanceCount _output_get_7) 1)))
      (for _index (range 0 _output_get_8)
        (bind _output_get_9 (Variables|Default|SetInstanceIndex _index))
        (bind _output_get_10 (Variables|Default|SetMeshTransform (.OutInstanceTransform (Components|InstancedStaticMesh|GetInstanceTransform (Variables|Default|GetInstancedStaticMesh) _output_get_9 false))))
        (Variables|Default|SetRelativeTransform (Class|KismetMathLibrary|ConvertTransformtoRelative (Variables|Default|GetBuildingPosition) _output_get_10))
        (Development|PrintString (Utilities|String|JoinStringArray (Utilities|Array|MakeArray (Utilities|String|ToString(Integer) _output_get_9) (Utilities|String|ToString(Float) (.x (.location (Variables|Default|GetRelativeTransform)))) (Utilities|String|ToString(Float) (.y (.location (Variables|Default|GetRelativeTransform)))) (Utilities|String|ToString(Float) (.z (.location (Variables|Default|GetRelativeTransform)))) (Utilities|String|ToString(Float) (.roll (.rotation (Variables|Default|GetRelativeTransform)))) (Utilities|String|ToString(Float) (.pitch (.rotation (Variables|Default|GetRelativeTransform)))) (Utilities|String|ToString(Float) (.yaw (.rotation (Variables|Default|GetRelativeTransform)))) (Utilities|String|ToString(Float) (.x (.scale (Variables|Default|GetRelativeTransform)))) (Utilities|String|ToString(Float) (.y (.scale (Variables|Default|GetRelativeTransform)))) (Utilities|String|ToString(Float) (.z (.scale (Variables|Default|GetRelativeTransform))))) ":"))))))

(fn ConstructionScript)