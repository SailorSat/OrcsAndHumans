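; Taxi actor that loops along a track's spline, stopping to wait at points marked with the Linear point type.
; A tick-driven four-state machine waits, accelerates, cruises and brakes ahead of the next stop, with depart and dock sounds off dedicated servers.
; Each tick derives position and yaw from spline distance.
; At each stop the server calls ForceReplication to push the full movement state.
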(event Custom|ForceReplication
  (params (SpeedCurrent :type Float%20%28single-precision%29) (SpeedMax :type Float%20%28single-precision%29) (Status :type Integer) (WaitTime :type Float%20%28single-precision%29) (WaitTimeCurrent :type Float%20%28single-precision%29) (Position :type Float%20%28single-precision%29) (NextPoint :type Integer) (SpeedDelta :type Float%20%28single-precision%29) (WaitDistance :type Float%20%28single-precision%29) (SpeedFactor :type Float%20%28single-precision%29))
  (Variables|Default|SetSpeedCurrent SpeedCurrent)
  (Variables|Default|SetSpeedMax SpeedMax)
  (Variables|Default|SetStatus Status)
  (Variables|Default|SetWaitTime WaitTime)
  (Variables|Default|SetWaitTimeCurrent WaitTimeCurrent)
  (Variables|Default|SetPosition Position)
  (Variables|Default|SetNextPoint NextPoint)
  (Variables|Default|SetSpeedDelta SpeedDelta)
  (Variables|Default|SetWaitDistance WaitDistance)
  (Variables|Default|SetSpeedFactor SpeedFactor))

(event EventBeginPlay
  (bind _track (Variables|Default|GetTrack))
  (Utilities|IsValid _track
    (:Is%20Valid
      (Variables|Default|SetSpline (Variables|/Game/Mods/OrcsAndHumans/Taxi/BP_TaxiPath.BP_TaxiPath_C|GetSpline _track))
      (Actor|Tick|SetActorTickEnabled true)
      (if (Networking|IsServer)
        (CallFunction|FindNextWait)))))

(event EventTick
  (params (DeltaSeconds :type Float%20%28single-precision%29))
  (bind _speedmax (Variables|Default|GetSpeedMax))
  (bind _position (Variables|Default|GetPosition))
  (bind _waitdistance (Variables|Default|GetWaitDistance))
  (CallFunction|UpdatePosition DeltaSeconds)
  (switch int (Variables|Default|GetStatus)
    (:0
      (if (> (Variables|Default|GetWaitTimeCurrent) 0.0)
        (Variables|Default|SetWaitTimeCurrent (- (Variables|Default|GetWaitTimeCurrent) DeltaSeconds))
        (else
          (Variables|Default|SetStatus 1)
          (if (not (Networking|IsDedicatedServer))
            (Class|AudioFunctionLibrary|PlaySoundatLocation (Variables|Default|GetDepartSound) (Transformation|GetActorLocation) "0, 0, 0" 1.0 1.0 0.0 "/Game/Sound/Attenuations/Att_Avatar_Giant.Att_Avatar_Giant" "/Game/Sound/Concurrencies/3D_Env_Life_General.3D_Env_Life_General")))))
    (:1
      (if (< (Variables|Default|GetSpeedCurrent) _speedmax)
        (Variables|Default|SetSpeedCurrent (+ (Variables|Default|GetSpeedCurrent) (Variables|Default|GetSpeedDelta)))
        (else
          (Variables|Default|SetSpeedCurrent _speedmax)
          (Variables|Default|SetStatus 2))))
    (:2
      (Utilities|And+Branch (> _waitdistance _position) (< (- _waitdistance _position) (* (Variables|Default|GetSpeedCurrent) 0.5 (Variables|Default|GetSpeedFactor)))
        (:True
          (Variables|Default|SetStatus 3)
          (if (not (Networking|IsDedicatedServer))
            (Class|AudioFunctionLibrary|PlaySoundatLocation (Variables|Default|GetDockSound) (Transformation|GetActorLocation) "0, 0, 0" 1.0 1.0 0.0 "/Game/Sound/Attenuations/Att_Avatar_Giant.Att_Avatar_Giant" "/Game/Sound/Concurrencies/3D_Env_Life_General.3D_Env_Life_General")))))
    (:3
      (if (> (Variables|Default|GetSpeedCurrent) 0.0)
        (Variables|Default|SetSpeedCurrent (- (Variables|Default|GetSpeedCurrent) (Variables|Default|GetSpeedDelta)))
        (else
          (Variables|Default|SetWaitTimeCurrent (Variables|Default|GetWaitTime))
          (Variables|Default|SetSpeedCurrent 0.0)
          (Variables|Default|SetStatus 0)
          (CallFunction|FindNextWait)
          (if (Networking|IsServer)
            (CallFunction|ForceReplication (Variables|Default|GetSpeedCurrent) (Variables|Default|GetSpeedMax) (Variables|Default|GetStatus) (Variables|Default|GetWaitTime) (Variables|Default|GetWaitTimeCurrent) (Variables|Default|GetPosition) (Variables|Default|GetNextPoint) (Variables|Default|GetSpeedDelta) (Variables|Default|GetWaitDistance) (Variables|Default|GetSpeedFactor))))))))

(fn ConstructionScript)

(fn FindNextWait
  (bind _spline (Variables|Default|GetSpline))
  (while (Utilities|Enum|NotEqual(Enum) "Linear" (Class|SplineComponent|GetSplinePointType (Variables|Default|GetSpline) (Variables|Default|GetNextPoint)))
    (Variables|Default|SetNextPoint (Math|Integer|%(Integer) (+ (Variables|Default|GetNextPoint) 1) (Spline|GetNumberOfSplinePoints _spline))))
  (if (== (Variables|Default|GetNextPoint) 0)
    (Variables|Default|SetWaitDistance (Spline|GetSplineLength _spline))
    (else
      (bind _output_get (Variables|Default|SetWaitDistance (Spline|GetDistanceAlongSplineatSplinePoint _spline (Variables|Default|GetNextPoint))))))
  (Development|PrintString (Utilities|String|Append "Next Wait at: " (Utilities|String|ToString(Float) _output_get)))
  (Variables|Default|SetNextPoint (Math|Integer|%(Integer) (+ (Variables|Default|GetNextPoint) 1) (Spline|GetNumberOfSplinePoints _spline))))

(fn UpdatePosition
  (params (DeltaSeconds :type Float%20%28single-precision%29))
  (bind _spline (Variables|Default|GetSpline))
  ;[1 1 1] Calculate Speed Delta
  (Variables|Default|SetSpeedDelta (/ (* DeltaSeconds (Variables|Default|GetSpeedMax)) (Variables|Default|GetSpeedFactor)))
  ;[1 1 1] Calculate Position and update Location & Rotation
  (bind _output_get (Variables|Default|SetPosition (Math|Float|%(Float) (+ (* DeltaSeconds (Variables|Default|GetSpeedCurrent)) (Variables|Default|GetPosition)) (Spline|GetSplineLength _spline))))
  (Transformation|SetActorLocationAndRotation (Spline|GetLocationatDistanceAlongSpline _spline _output_get "World") (Math|Rotator|MakeRotator 0.0 0.0 (.yaw (Math|Conversions|RotationFromXVector (Spline|GetTangentatDistanceAlongSpline _spline _output_get "World")))))
  (return))