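; OAH_ManualSpawnPoint is a spawn point that swaps its wildlife and human spawn options according to which mods are loaded.
; On BeginPlay it finds the OAH_PreLoad_ModController and scans its ModSpawns entries against the loaded and test mod lists.
; The first match replaces WildlifeOptions and HumanOptions entirely.
; The replacement runs before parent BeginPlay, and without a match or valid controller the existing options remain.
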(event EventBeginPlay
  (CallFunction|ReplaceSpawns)
  (|CallParentFunction))

(fn ConstructionScript
  (|CallParentFunction))

(fn ReplaceSpawns
  (bind _wildlifeoptions (Variables|Default|GetWildlifeOptions))
  (bind _humanoptions (Variables|Default|GetHumanOptions))
  (bind _outactors (Actor|GetAllActorsOfClass "/Game/Mods/OrcsAndHumans/PreLoad/OAH_PreLoad_ModController.OAH_PreLoad_ModController_C"))
  (bind _output_get (LocalVariables|SetModController (Utilities|Array|Get(acopy) _outactors)))
  (Utilities|IsValid _output_get
    (:Is%20Valid
      (for _array_element (Variables|Default|GetModSpawns)
        (Utilities|Or+Branch (Utilities|Set|Contains (Variables|/Game/Mods/OrcsAndHumans/PreLoad/OAH_PreLoad_ModController.OAH_PreLoad_ModController_C|GetLoadedMods (LocalVariables|GetModController)) (.modid _array_element)) (Utilities|Set|Contains (Variables|/Game/Mods/OrcsAndHumans/PreLoad/OAH_PreLoad_ModController.OAH_PreLoad_ModController_C|GetLoadedTestMods (LocalVariables|GetModController)) (.testmodid _array_element))
          (:True
            (Utilities|Array|Clear _wildlifeoptions)
            (Utilities|Array|AppendArray _wildlifeoptions (.wildlifeoptions _array_element))
            (Utilities|Array|Clear _humanoptions)
            (Utilities|Array|AppendArray _humanoptions (.humanoptions _array_element))
            (return))))
      (return))
    (:Is%20Not%20Valid
      (return))))