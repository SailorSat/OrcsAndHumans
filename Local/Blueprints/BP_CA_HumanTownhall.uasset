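; BP_CA_HumanTownhall is a human town hall building with faction-specific looks and a working clock.
; The construction script batch-swaps the mesh's slot materials from a per-faction map chosen by FactionTemplate.
; Outside dedicated servers, BeginPlay finds BP_TimeOfDayManager and, if found, enables tick, which rotates the hour and minute hands to match the in-game time.
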(event EventBeginPlay
  (if (not (Networking|IsDedicatedServer))
    (bind _outactors (Actor|GetAllActorsOfClass "/Game/Systems/BP_TimeOfDayManager.BP_TimeOfDayManager_C"))
    (Utilities|IsValid (Utilities|Array|Get(acopy) _outactors)
      (:Is%20Valid
        (Variables|Default|SetTimeOfDayManager (Utilities|Array|Get(acopy) _outactors))
        (Actor|Tick|SetActorTickEnabled true)))))

(event EventTick
  (params (DeltaSeconds :type Float%20%28single-precision%29))
  (bind _returnvalue (Class|ConanTimeOfDayManager|GetTimeOfDay (Variables|Default|GetTimeOfDayManager)))
  (Transformation|SetRelativeRotation (Variables|Default|GetArrowH) (Math|Rotator|MakeRotator 0.0 0.0 (* (Math|Float|%(Float) _returnvalue 12.0) 3e+01)) false false)
  (Transformation|SetRelativeRotation (Variables|Default|GetArrowM) (Math|Rotator|MakeRotator 0.0 0.0 (* (Math|Float|%(Float) _returnvalue 1.0) 3.6e+02)) false false))

(fn ConstructionScript
  (bind _staticmesh (Variables|Default|GetStaticMesh))
  (switch Utilities|FlowControl|Switch|SwitchonE_HumanFaction (Variables|Default|GetFactionTemplate)
    (:NewEnumerator1
      (CallFunction|BatchUpdateMaterials _staticmesh (LocalVariables|GetMapWestfall)))
    (:NewEnumerator2
      (CallFunction|BatchUpdateMaterials _staticmesh (LocalVariables|GetMapDuskwood)))
    (:NewEnumerator3
      (CallFunction|BatchUpdateMaterials _staticmesh (LocalVariables|GetMapRedridge)))
    (:NewEnumerator4
      (CallFunction|BatchUpdateMaterials _staticmesh (LocalVariables|GetMapKarazhan)))
    (:NewEnumerator10
      (CallFunction|BatchUpdateMaterials _staticmesh (LocalVariables|GetMapStratholme)))
    (:NewEnumerator11
      (CallFunction|BatchUpdateMaterials _staticmesh (LocalVariables|GetMapHearthglen)))))