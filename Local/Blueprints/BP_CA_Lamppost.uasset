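; Lamppost actor that lights up at night and switches off by day, toggling its point light, particle effect and audio volume.
; Outside dedicated servers, BeginPlay finds the BP_TimeOfDayManager, enables tick at a randomized 30–45 second interval and runs an immediate check.
; Each check reads the time of day, treats 5 to 20 as daytime, and calls TurnOn or TurnOff only when the IsActive state must change.
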(event Custom|ManualTick
  (bind _returnvalue (Class|ConanTimeOfDayManager|GetTimeOfDay (Variables|Default|GetTimeOfDayManager)))
  (if (Math|Float|InRange(Float) _returnvalue 5.0 2e+01) ; is daytime?
    (if (Variables|Default|GetIsActive)
      (Variables|Default|SetIsActive false)
      (CallFunction|TurnOff))
    (elif (not (Variables|Default|GetIsActive))
      (Variables|Default|SetIsActive true)
      (CallFunction|Turnon))))

(event Custom|TurnOff
  (Class|ConanAudioComponent|SetVolumeMultiplier (Variables|Default|GetConanAudio) 0.0)
  (Components|Activation|Deactivate (Variables|Default|GetParticleSystem))
  (Rendering|SetVisibility (Variables|Default|GetPointLight) false true))

(event Custom|TurnOn
  (Class|ConanAudioComponent|SetVolumeMultiplier (Variables|Default|GetConanAudio) 1.0)
  (Components|Activation|Activate (Variables|Default|GetParticleSystem) true)
  (Rendering|SetVisibility (Variables|Default|GetPointLight) true true))

(event EventBeginPlay
  (if (not (Networking|IsDedicatedServer))
    (bind _outactors (Actor|GetAllActorsOfClass "/Game/Systems/BP_TimeOfDayManager.BP_TimeOfDayManager_C"))
    (Utilities|IsValid (Utilities|Array|Get(acopy) _outactors)
      (:Is%20Valid
        (Variables|Default|SetTimeOfDayManager (Utilities|Array|Get(acopy) _outactors))
        (Actor|Tick|SetActorTickEnabled true)
        (Actor|Tick|SetActorTickInterval (Math|Random|RandomFloatinRange 3e+01 45.0))
        (CallFunction|ManualTick)))))

(event EventTick
  (params (DeltaSeconds :type Float%20%28single-precision%29))
  (bind _returnvalue (Class|ConanTimeOfDayManager|GetTimeOfDay (Variables|Default|GetTimeOfDayManager)))
  (if (Math|Float|InRange(Float) _returnvalue 5.0 2e+01) ; is daytime?
    (if (Variables|Default|GetIsActive)
      (Variables|Default|SetIsActive false)
      (CallFunction|TurnOff))
    (elif (not (Variables|Default|GetIsActive))
      (Variables|Default|SetIsActive true)
      (CallFunction|Turnon))))

(fn ConstructionScript)