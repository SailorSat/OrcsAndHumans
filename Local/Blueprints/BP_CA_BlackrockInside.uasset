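; Blackrock interior environment actor that procedurally builds a bridge and a ring from two splines.
; Its construction script divides each spline by MeshLength and adds a spline mesh component per segment, fitted to the spline's locations and tangents.
; Segments overlap by a fixed offset: bridge pieces start early and ring pieces end late.
; A ring piece that would pass the spline's end wraps to just past the start, closing the loop.
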(fn ConstructionScript
  (CallFunction|BuildBridgefromSpline)
  (CallFunction|BuildRingfromSpline))

(fn BuildBridgefromSpline
  (bind _meshlength (LocalVariables|GetMeshLength))
  (bind _bridge_spline (Variables|Default|Getbridge_spline))
  (bind _output_get (LocalVariables|SetSegmentCount (Math|Float|Truncate (/ (Spline|GetSplineLength (Variables|Default|Getbridge_spline)) (LocalVariables|GetMeshLength)))))
  (for _index (range 0 _output_get)
    (bind _output_get_2 (LocalVariables|SetStartIndex _index))
    (bind _output_get_3 (LocalVariables|SetEndIndex (+ _output_get_2 1)))
    (bind _output_get_4 (LocalVariables|SetStartDistance (* _output_get_2 _meshlength)))
    (bind _output_get_5 (LocalVariables|SetEndDistance (* _output_get_3 _meshlength)))
    (bind _returnvalue (AddComponent|AddSplineMeshComponent false (Transformation|GetRelativeTransform _bridge_spline)))
    (SplineMesh|SetStartandEnd _returnvalue (Spline|GetLocationatDistanceAlongSpline _bridge_spline (- _output_get_4 256.0) "Local") (Spline|GetTangentatDistanceAlongSpline _bridge_spline (- _output_get_4 256.0) "Local") (Spline|GetLocationatDistanceAlongSpline _bridge_spline _output_get_5 "Local") (Spline|GetTangentatDistanceAlongSpline _bridge_spline _output_get_5 "Local") true :!class /Script/Engine.SplineMeshComponent)))

(fn BuildRingfromSpline
  (bind _meshlength (LocalVariables|GetMeshLength))
  (bind _ring_spline (Variables|Default|Getring_spline))
  (bind _output_get (LocalVariables|SetSegmentCount (Math|Float|Truncate (/ (Spline|GetSplineLength (Variables|Default|Getring_spline)) (LocalVariables|GetMeshLength)))))
  (for _index (range 0 _output_get)
    (bind _output_get_2 (LocalVariables|SetStartIndex _index))
    (bind _output_get_3 (LocalVariables|SetEndIndex (+ _output_get_2 1)))
    (bind _output_get_4 (LocalVariables|SetStartDistance (* _output_get_2 _meshlength)))
    (bind _output_get_5 (LocalVariables|SetEndDistance (* _output_get_3 _meshlength)))
    (bind _returnvalue (AddComponent|AddSplineMeshComponent false (Transformation|GetRelativeTransform _ring_spline)))
    (if (> _output_get_5 (Spline|GetSplineLength _ring_spline))
      (SplineMesh|SetStartandEnd _returnvalue (Spline|GetLocationatDistanceAlongSpline _ring_spline _output_get_4 "Local") (Spline|GetTangentatDistanceAlongSpline _ring_spline _output_get_4 "Local") (Spline|GetLocationatDistanceAlongSpline _ring_spline 256.0 "Local") (Spline|GetTangentatDistanceAlongSpline _ring_spline 256.0 "Local") true :!class /Script/Engine.SplineMeshComponent)
      (else
        (SplineMesh|SetStartandEnd _returnvalue (Spline|GetLocationatDistanceAlongSpline _ring_spline _output_get_4 "Local") (Spline|GetTangentatDistanceAlongSpline _ring_spline _output_get_4 "Local") (Spline|GetLocationatDistanceAlongSpline _ring_spline (+ _output_get_5 256.0) "Local") (Spline|GetTangentatDistanceAlongSpline _ring_spline (+ _output_get_5 256.0) "Local") true :!class /Script/Engine.SplineMeshComponent)))))