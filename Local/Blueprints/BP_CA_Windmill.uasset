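; Windmill actor that turns and spins in response to the level's wind.
; On BeginPlay, outside dedicated servers, it caches the first WindDirectionalSource found and enables tick.
; Each tick, Top yaws to the wind's yaw plus a half turn, and Rotator rolls at a rate scaled by wind speed.
; A cosine-based GetRotationModifier helper is defined but not called in these graphs.
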(event EventTick
  (params (DeltaSeconds :type Float%20%28single-precision%29))
  (bind _windsource (Variables|Default|GetWindSource))
  (Transformation|SetWorldRotation (Variables|Default|GetTop) (Math|Rotator|MakeRotator 0.0 0.0 (+ (.yaw (Transformation|GetActorRotation _windsource)) 1.8e+02)) false false)
  (Transformation|AddLocalRotation (Variables|Default|GetRotator) (Math|Rotator|MakeRotator (* DeltaSeconds (Variables|/Script/Engine.WindDirectionalSourceComponent|GetSpeed (Variables|/Script/Engine.WindDirectionalSource|GetComponent _windsource)) -3.6e+02) 0.0 0.0) false false))

(event EventBeginPlay
  (if (not (Networking|IsDedicatedServer))
    (bind _outactors (Actor|GetAllActorsOfClass "/Script/Engine.WindDirectionalSource"))
    (Utilities|IsValid (Utilities|Array|Get(acopy) _outactors)
      (:Is%20Valid
        (Variables|Default|SetWindSource (Utilities|Array|Get(acopy) _outactors))
        (Actor|Tick|SetActorTickEnabled true)))))

(fn ConstructionScript)

(fn GetRotationModifier
  (params (Delta :type Float%20%28single-precision%29) (Current :type Float%20%28single-precision%29) (Target :type Float%20%28single-precision%29))
  (return (* (- (Math|Trig|Cos(Degrees) Target) (Math|Trig|Cos(Degrees) Current)) 1.8e+02)))