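; Spline-driven Blueprint that builds canal sections, judging by its name, along an editable path.
; The construction script splits each stretch between spline points into equal segments no longer than the section length, adding a spline mesh component for each.
; Segment ends extend slightly to overlap, and tangents are clamped to the section length.
; Closed loops get their final stretch filled; an unused debug one-mesh-per-stretch variant remains.
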(event EventBeginPlay)

(fn ConstructionScript
  (bind _sectionlength (Variables|Default|GetSectionLength))
  (bind _spline (Variables|Default|GetSpline))
  (bind _spline_2 (Variables|Default|GetSpline))
  (bind _returnvalue (Spline|GetNumberOfSplinePoints _spline_2))
  (for _index (range 0 (- _returnvalue 2))
    (bind _output_get (LocalVariables|SetStartIndex _index))
    (bind _output_get_2 (LocalVariables|SetEndIndex (+ _index 1)))
    (bind _output_get_3 (LocalVariables|SetStartDistance (Spline|GetDistanceAlongSplineatSplinePoint _spline_2 _output_get)))
    (bind _output_get_4 (LocalVariables|SetEndDistance (Spline|GetDistanceAlongSplineatSplinePoint _spline_2 _output_get_2)))
    (bind _output_get_5 (LocalVariables|SetSegmentDistance (- _output_get_4 _output_get_3)))
    (bind _output_get_6 (LocalVariables|SetSegmentCount (+ (Math|Float|Truncate (/ _output_get_5 (Variables|Default|GetSectionLength))) 1)))
    (LocalVariables|SetSegmentLength (/ _output_get_5 (Math|Conversions|ToFloat(Integer) (+ (Math|Float|Truncate (/ _output_get_5 (Variables|Default|GetSectionLength))) 1))))
    (for _index_2 (range 1 _output_get_6)
      (bind _returnvalue_2 (AddComponent|AddSplineMeshComponent false))
      (SplineMesh|SetForwardAxis _returnvalue_2 "X" true)
      (SplineMesh|SetStartandEnd _returnvalue_2 (Spline|GetLocationatDistanceAlongSpline _spline (+ (* (- _index_2 1) (LocalVariables|GetSegmentLength)) (LocalVariables|GetStartDistance)) "Local") (Math|Vector|ClampVectorSize (Spline|GetTangentatDistanceAlongSpline _spline (+ (* (- _index_2 1) (LocalVariables|GetSegmentLength)) (LocalVariables|GetStartDistance)) "Local") 0.0 _sectionlength) (Spline|GetLocationatDistanceAlongSpline _spline (+ (+ (LocalVariables|GetStartDistance) (* _index_2 (LocalVariables|GetSegmentLength))) 3e+01) "Local") (Math|Vector|ClampVectorSize (Spline|GetTangentatDistanceAlongSpline _spline (+ (+ (LocalVariables|GetStartDistance) (* _index_2 (LocalVariables|GetSegmentLength))) 3e+01) "Local") 0.0 _sectionlength) true :!class /Script/Engine.SplineMeshComponent)))
  (if (Class|SplineComponent|IsClosedLoop _spline_2)
    (LocalVariables|SetStartIndex (- _returnvalue 1))
    (LocalVariables|SetEndIndex _returnvalue)
    (bind _output_get_7 (LocalVariables|SetStartDistance (Spline|GetDistanceAlongSplineatSplinePoint _spline_2 _output_get)))
    (bind _output_get_8 (LocalVariables|SetEndDistance (Spline|GetDistanceAlongSplineatSplinePoint _spline_2 _output_get_2)))
    (bind _output_get_9 (LocalVariables|SetSegmentDistance (- _output_get_8 _output_get_7)))
    (bind _output_get_10 (LocalVariables|SetSegmentCount (+ (Math|Float|Truncate (/ _output_get_9 (Variables|Default|GetSectionLength))) 1)))
    (LocalVariables|SetSegmentLength (/ _output_get_9 (Math|Conversions|ToFloat(Integer) (+ (Math|Float|Truncate (/ _output_get_9 (Variables|Default|GetSectionLength))) 1))))
    (for _index_3 (range 1 _output_get_10)
      (bind _returnvalue_3 (AddComponent|AddSplineMeshComponent false))
      (SplineMesh|SetForwardAxis _returnvalue_3 "X" true)
      (SplineMesh|SetStartandEnd _returnvalue_3 (Spline|GetLocationatDistanceAlongSpline _spline (+ (* (- _index_3 1) (LocalVariables|GetSegmentLength)) (LocalVariables|GetStartDistance)) "Local") (Math|Vector|ClampVectorSize (Spline|GetTangentatDistanceAlongSpline _spline (+ (* (- _index_3 1) (LocalVariables|GetSegmentLength)) (LocalVariables|GetStartDistance)) "Local") 0.0 _sectionlength) (Spline|GetLocationatDistanceAlongSpline _spline (+ (+ (LocalVariables|GetStartDistance) (* _index_3 (LocalVariables|GetSegmentLength))) 3e+01) "Local") (Math|Vector|ClampVectorSize (Spline|GetTangentatDistanceAlongSpline _spline (+ (+ (LocalVariables|GetStartDistance) (* _index_3 (LocalVariables|GetSegmentLength))) 3e+01) "Local") 0.0 _sectionlength) true :!class /Script/Engine.SplineMeshComponent))))