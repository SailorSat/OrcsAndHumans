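; Meteor projectile Blueprint that supplies the grounded meteor actor left behind by the projectile.
; SpawnGroundedActor line-traces a short distance straight down on Visibility so the meteor sits embedded in the ground, falling back to the projectile's own transform on a miss.
; It always spawns OAH_MeteorGrounded with the projectile's rotation and scale, calls Initialize on it and returns it.
; The event graph holds no active logic.
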(event EventBeginPlay
  (|CallParentFunction))

(event Collision|EventActorBeginOverlap
  (params (OtherActor :type Actor%20Object%20Reference)))

(event EventTick
  (params (DeltaSeconds :type Float%20%28single-precision%29)))

(fn ConstructionScript
  (|CallParentFunction))

(fn SpawnGroundedActor
  (bind _returnvalue (Transformation|GetActorTransform))
  (bind _returnvalue_2 (Transformation|GetActorTransform))
  (bind _location (Math|Transform|BreakTransform _returnvalue_2))
  (bind (_location_2 _rotation _scale) (Math|Transform|BreakTransform _returnvalue))
  ;[0.62 0 0] Make sure projectile gets embedded in the ground.
  (bind (_outhit _returnvalue_3) (Collision|LineTraceByChannel _location (+ _location (* "0, 0,-1.000000" 2e+02)) "TraceTypeQuery1" false 0 "None"))
  (bind _returnvalue_4 (Game|SpawnActorfromClass "/Game/Mods/OrcsAndHumans/Blueprints/OAH_MeteorGrounded.OAH_MeteorGrounded_C" (select _returnvalue_3 (Math|Transform|MakeTransform (.Location (Collision|BreakHitResult _outhit)) _rotation _scale) (Transformation|GetActorTransform)) "AlwaysSpawn" 0 0))
  (Default|Initialize _returnvalue_4)
  (return _returnvalue_4))