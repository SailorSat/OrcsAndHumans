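; Server-authoritative teleport trigger volume that moves players to a linked destination.
; Overlap events on the TriggerBox are enabled only on the server at BeginPlay.
; When a BasePlayerChar enters, its FunCombat_PlayerController teleports it to a random point inside the TeleportDestination's ReceiverBox, matching that box's rotation and forcing the teleport on clients.
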(event OnComponentBeginOverlap(TriggerBox)
  (params (OverlappedComponent :type Primitive%20Component%20Object%20Reference) (OtherActor :type Actor%20Object%20Reference) (OtherComp :type Primitive%20Component%20Object%20Reference) (OtherBodyIndex :type Integer) (bFromSweep :type Boolean) (SweepResult :type Hit%20Result%20Structure%20%28by%20ref%29))
  (bind _teleportdestination (Variables|Default|GetTeleportDestination))
  (bind _receiverbox (Variables|OAH_InstanceTeleport_C|GetReceiverBox _teleportdestination))
  (Utilities|Casting|CastToBasePlayerChar OtherActor)
  (bind _asfun_combat_player_controller (Utilities|Casting|CastToFunCombat_PlayerController (CallFunction|GetControllerfromActor OtherActor)))
  (Class|ConanPlayerController|TeleportPlayerServer _asfun_combat_player_controller (Class|FuncomGenericLibrary|GetRandomPointinBox _receiverbox) (Transformation|GetWorldRotation _receiverbox) false false true false))

(event EventBeginPlay
  (bind _triggerbox (Variables|Default|GetTriggerBox))
  (if (Networking|IsServer)
    (Variables|/Script/Engine.PrimitiveComponent|SetbGenerateOverlapEvents _triggerbox true)
    (else
      (Variables|/Script/Engine.PrimitiveComponent|SetbGenerateOverlapEvents _triggerbox false))))

(fn ConstructionScript)