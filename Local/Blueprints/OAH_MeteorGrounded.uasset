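; OAH_MeteorGrounded is a meteor Blueprint that randomizes its appearance when play begins.
; On the server only, BeginPlay rolls one random index and uses it to set both the core visual mesh and the core destructible mesh from parallel arrays, keeping the pair matched.
; The construction script only calls its parent.
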(event EventBeginPlay
  (if (Networking|IsServer)
    (bind _output_get (Variables|Default|SetRND (Math|Random|RandomIntegerinRange 0 4)))
    (Variables|Default|SetCoreVisualMesh (Utilities|Array|Get(acopy) (Variables|Default|GetVisualMeshes) _output_get))
    (Variables|Default|SetCoreDestructibleMesh (Utilities|Array|Get(acopy) (Variables|Default|GetDestructibleMeshes) _output_get))))

(fn ConstructionScript
  (|CallParentFunction))