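; Armor display mannequin that builds a character from a customization Layout and plays a looping idle animation.
; On BeginPlay it applies the layout, then swaps meshes, materials and animation in steps spaced by short delays.
; Name-keyed replacement maps supply asset paths loaded at runtime, with dynamic materials matched by parent name.
; The male or female idle is also loaded by path, skipping dedicated servers.
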(event Custom|UpdateLayout
  (Class|CharacterCustomizationComponent|SetCharacterLayout (Variables|Default|GetCharCustomization) (Variables|Default|GetLayout) false true false)
  (Utilities|FlowControl|Delay 0.5)
  (CallFunction|UpdateMeshes))

(event Custom|UpdateAnimation
  (if (not (Networking|IsDedicatedServer))
    (bind _returnvalue (Class|FuncomGenericLibrary|LoadAssetfromPath (Utilities|String|SelectString "/Game/DLC/Special/s1c3/Characters/mannequin/Animations/A_mannequin_idle_01_F.A_mannequin_idle_01_F" "/Game/DLC/Special/s1c3/Characters/mannequin/Animations/A_mannequin_idle_01_M.A_mannequin_idle_01_M" (.isfemale (.boolparams (Variables|Default|GetLayout))))))
    (bind _asanim_sequence_base (Utilities|Casting|CastToAnimSequenceBase _returnvalue)
      (:then
        (bind _output_get (Variables|Default|SetAnimation _asanim_sequence_base)))
      (:CastFailed
        _))
    (Components|Animation|PlayAnimation (Variables|SkeletalMeshActor|GetSkeletalMeshComponent) _output_get true)))

(event Custom|UpdateMaterials
  (CallFunction|ReplaceMaterials)
  (Utilities|FlowControl|Delay 0.5)
  (CallFunction|UpdateAnimation))

(event Custom|UpdateMeshes
  (CallFunction|ReplaceMeshes)
  (Utilities|FlowControl|Delay 0.5)
  (CallFunction|UpdateMaterials))

(event EventBeginPlay
  (CallFunction|UpdateLayout))

(fn ConstructionScript
  (Class|CharacterCustomizationComponent|SetMasterSkeletalMeshComponent (Variables|Default|GetCharCustomization) (Variables|SkeletalMeshActor|GetSkeletalMeshComponent) false))

(fn ReplaceMeshes
  (bind _output_get (LocalVariables|SetMeshComponentList (Actor|GetComponentsByClass "/Script/Engine.SkeletalMeshComponent")))
  (for _array_element _output_get
    (bind _output_get_2 (LocalVariables|SetMeshComponentCurrent _array_element))
    (if (.ReturnValue (Utilities|Map|Find (Variables|Default|GetMeshReplacement) (Utilities|GetObjectName (Variables|/Script/Engine.SkinnedMeshComponent|GetSkeletalMesh _output_get_2))))
      (bind _returnvalue (Class|FuncomGenericLibrary|LoadAssetfromPath (.Value (Utilities|Map|Find (Variables|Default|GetMeshReplacement) (Utilities|GetObjectName (Variables|/Script/Engine.SkinnedMeshComponent|GetSkeletalMesh _output_get_2))))))
      (Utilities|IsValid _returnvalue
        (:Is%20Valid
          (bind _asskeletal_mesh (Utilities|Casting|CastToSkeletalMesh _returnvalue))
          (Class|SkinnedMeshComponent|SetSkeletalMesh _output_get_2 _asskeletal_mesh false)))))
  (return))

(fn ReplaceMaterials
  (bind _output_get (LocalVariables|SetMeshComponentList (Actor|GetComponentsByClass "/Script/Engine.SkeletalMeshComponent")))
  (for _array_element _output_get
    (bind _output_get_2 (LocalVariables|SetMeshComponentCurrent _array_element))
    (bind _output_get_3 (LocalVariables|SetMaterialNum (Rendering|Material|GetNumMaterials _output_get_2)))
    (for _index (range 0 _output_get_3)
      (bind _output_get_4 (LocalVariables|SetMaterialIndex _index))
      (bind _output_get_5 (LocalVariables|SetMaterialCurrent (Rendering|Material|GetMaterial (LocalVariables|GetMeshComponentCurrent) _output_get_4)))
      (LocalVariables|SetMaterialName (Utilities|GetDisplayName _output_get_5))
      (bind _asmaterial_instance_dynamic (Utilities|Casting|CastToMaterialInstanceDynamic _output_get_5)
        (:then
          (bind _output_get_6 (LocalVariables|SetMaterialName (Utilities|GetDisplayName (Variables|/Script/Engine.MaterialInstance|GetParent _asmaterial_instance_dynamic)))))
        (:CastFailed
          _))
      (if (.ReturnValue (Utilities|Map|Find (Variables|Default|GetMaterialReplacement) _output_get_6))
        (bind _returnvalue (Class|FuncomGenericLibrary|LoadAssetfromPath (.Value (Utilities|Map|Find (Variables|Default|GetMaterialReplacement) _output_get_6))))
        (Utilities|IsValid _returnvalue
          (:Is%20Valid
            (bind _asmaterial_instance (Utilities|Casting|CastToMaterialInstance _returnvalue))
            (Rendering|Material|SetMaterial (LocalVariables|GetMeshComponentCurrent) (LocalVariables|GetMaterialIndex) _asmaterial_instance))))))
  (return))