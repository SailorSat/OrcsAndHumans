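; BP_CA_HumanBarn is a human barn building whose appearance varies by regional template, such as Westfall, Duskwood or Stratholme.
; Its Construction Script switches on FactionTemplate and picks that region's slot-to-material map.
; BatchUpdateMaterials applies the chosen map to the StaticMesh component, so one Blueprint covers all six regional variants.
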(fn ConstructionScript
  (bind _staticmesh (Variables|Default|GetStaticMesh))
  (switch Utilities|FlowControl|Switch|SwitchonE_HumanFaction (Variables|Default|GetFactionTemplate)
    (:NewEnumerator1
      (CallFunction|BatchUpdateMaterials _staticmesh (LocalVariables|GetMapWestfall)))
    (:NewEnumerator2
      (CallFunction|BatchUpdateMaterials _staticmesh (LocalVariables|GetMapDuskwood)))
    (:NewEnumerator3
      (CallFunction|BatchUpdateMaterials _staticmesh (LocalVariables|GetMapRedridge)))
    (:NewEnumerator4
      (CallFunction|BatchUpdateMaterials _staticmesh (LocalVariables|GetMapKarazhan)))
    (:NewEnumerator10
      (CallFunction|BatchUpdateMaterials _staticmesh (LocalVariables|GetMapStratholme)))
    (:NewEnumerator11
      (CallFunction|BatchUpdateMaterials _staticmesh (LocalVariables|GetMapHearthglen)))))