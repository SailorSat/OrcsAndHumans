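; BP_CA_TrollDrum03 is an interactable troll drum prop that triggers a sound when activated.
; Activation is forwarded to the BPBSCMulticastSound component, whose name indicates the sound is multicast to clients.
; The other interactable functions are stubs that report no looting, commanding, UI modules, default action or display text, and never disable activation or the menu.
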(event EventInteractableActivate
  (params (Component :type Primitive%20Component%20Object%20Reference) (Instigator :type Player%20Controller%20Object%20Reference) (HitIndex :type Integer) (TriggeredFromRadialWheel :type Boolean))
  (Default|InteractableActivate (Variables|Default|GetBP_BSC_MulticastSound) 0 0 0 false))

(fn ConstructionScript)

(fn InteractableActivateDisabled
  (params (InteractingCharacter :type Conan%20Character%20Object%20Reference))
  (return false))

(fn InteractableCanbeLooted
  (params (InteractingCharacter :type Conan%20Character%20Object%20Reference))
  (return false))

(fn InteractableDefaultAction
  (return "" 0))

(fn InteractableGetRepairUIModuleName
  (return "None"))

(fn InteractableGetSimpleDisplayText
  (return ""))

(fn InteractableGetUIModuleName
  (return "None"))

(fn InteractableMenuDisabled
  (params (InteractingCharacter :type Conan%20Character%20Object%20Reference))
  (return false))

(fn InteractableShouldCommand
  (return false))