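; BP_CA_Lamppost_2 is a switchable lamppost that extends a parent Blueprint with an emissive glow.
; On BeginPlay it creates a dynamic material instance from the third material slot of StaticMesh1, then calls the parent.
; Its Turnon and TurnOff events call the parent versions, then set emissive scale, intensity and saturation on that material to show the lit or unlit state.
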(event EventTurnon
  (bind _material (Variables|Default|GetMaterial))
  (|CallParentFunction)
  (Rendering|Material|SetScalarParameterValue _material "EmissiveScale" 1.0 :!class /Script/Engine.MaterialInstanceDynamic)
  (Rendering|Material|SetScalarParameterValue _material "emissive_intensity_1" 29.209364 :!class /Script/Engine.MaterialInstanceDynamic)
  (Rendering|Material|SetScalarParameterValue _material "emissive_saturation" 0.0 :!class /Script/Engine.MaterialInstanceDynamic))

(event EventTurnOff
  (bind _material (Variables|Default|GetMaterial))
  (|CallParentFunction)
  (Rendering|Material|SetScalarParameterValue _material "EmissiveScale" 0.0 :!class /Script/Engine.MaterialInstanceDynamic)
  (Rendering|Material|SetScalarParameterValue _material "emissive_intensity_1" 0.0 :!class /Script/Engine.MaterialInstanceDynamic)
  (Rendering|Material|SetScalarParameterValue _material "emissive_saturation" 0.5 :!class /Script/Engine.MaterialInstanceDynamic))

(event EventBeginPlay
  (bind _staticmesh1 (Variables|Default|GetStaticMesh1))
  (bind _returnvalue (Rendering|Material|CreateDynamicMaterialInstance _staticmesh1 2 (Rendering|Material|GetMaterial _staticmesh1 2) :!class /Script/Engine.PrimitiveComponent))
  (Variables|Default|SetMaterial _returnvalue)
  (|CallParentFunction))

(fn ConstructionScript)