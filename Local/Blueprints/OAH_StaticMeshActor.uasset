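; OAH_StaticMeshActor is a static mesh actor that swaps in a mesh loaded at runtime or construction from the StaticMeshToLoad path.
; ReplaceMesh loads the asset with LoadAssetFromPath, checks that it is valid, casts it to StaticMesh and assigns it to the StaticMeshComponent.
; Both the Construction Script and BeginPlay call ReplaceMesh, so the mesh is applied on construction and again when play begins.
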(event Custom|ReplaceMesh
  (bind _returnvalue (Class|FuncomGenericLibrary|LoadAssetfromPath (Variables|Default|GetStaticMeshToLoad)))
  (Utilities|IsValid _returnvalue
    (:Is%20Valid
      (bind _asstatic_mesh (Utilities|Casting|CastToStaticMesh _returnvalue))
      (bind _returnvalue_2 (Components|StaticMesh|SetStaticMesh (Variables|Debug|GetStaticMeshComponent) _asstatic_mesh))
      (if _returnvalue_2
        _))))

(event EventBeginPlay
  (CallFunction|ReplaceMesh))

(fn ConstructionScript
  (CallFunction|ReplaceMesh))