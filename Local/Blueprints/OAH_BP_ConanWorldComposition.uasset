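; Conan world composition Blueprint that supplies the world positions around which level streaming happens, covering gameplay and character creation.
; GetStreamingPositions returns the controlled pawn's location when one exists.
; With a player controller but no pawn, it uses the cinematic camera plus any character creation helper, else the initial player start, else actors tagged for character creation.
; Controller, pawn, camera and helper references are found lazily and cached.
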(fn GetStreamingPositions
  (bind _returnvalue (Game|GetPlayerController 0))
  (bind _result (LocalVariables|GetResult))
  (Utilities|IsValid (Variables|Default|GetControlledPawn)
    (:Is%20Valid
      _)
    (:Is%20Not%20Valid
      (Utilities|IsValid (Variables|Default|GetPlayerController)
        (:Is%20Valid
          _)
        (:Is%20Not%20Valid
          (Utilities|IsValid _returnvalue
            (:Is%20Valid
              (bind _asconan_player_controller (Utilities|Casting|CastToConanPlayerController _returnvalue)
                (:then
                  (bind _output_get (Variables|Default|SetPlayerController _asconan_player_controller)))
                (:CastFailed
                  (return (LocalVariables|GetResult)))))
            (:Is%20Not%20Valid
              (return (LocalVariables|GetResult))))))
      (Utilities|IsValid (Pawn|GetControlledPawn _output_get)
        (:Is%20Valid
          (bind _output_get_2 (Variables|Default|SetControlledPawn (Pawn|GetControlledPawn _output_get))))
        (:Is%20Not%20Valid
          (Utilities|IsValid (Variables|Default|GetCinematicCamera)
            (:Is%20Valid
              _)
            (:Is%20Not%20Valid
              (bind _outactors (Actor|GetAllActorsOfClass "/Script/CinematicCamera.CineCameraActor"))
              (if (> (Utilities|Array|Length _outactors) 0)
                (Variables|Default|SetCinematicCamera (Utilities|Array|Get(acopy) _outactors))
                (else
                  (Utilities|IsValid (Variables|/Script/ConanSandbox.ConanPlayerController|GetInitialPlayerStart (Variables|Default|GetPlayerController))
                    (:Is%20Valid
                      (return (Utilities|Array|MakeArray (Transformation|GetActorLocation (Variables|/Script/ConanSandbox.ConanPlayerController|GetInitialPlayerStart (Variables|Default|GetPlayerController))))))
                    (:Is%20Not%20Valid
                      (bind _outactors_2 (Actor|GetAllActorswithTag (Variables|Default|GetCharacterCreationTag)))
                      (for _array_element _outactors_2
                        (Utilities|Array|Add _result (Transformation|GetActorLocation _array_element)))
                      (return _result)))))))
          (Utilities|IsValid (Variables|Default|GetCharacterCreationHelper)
            (:Is%20Valid
              _)
            (:Is%20Not%20Valid
              (bind _outactors_3 (Actor|GetAllActorsOfClass "/Game/Mods/OrcsAndHumans/CharacterCreation/OAH_CharacterCreationHelper.OAH_CharacterCreationHelper_C"))
              (if (> (Utilities|Array|Length _outactors_3) 0)
                (bind _output_get_3 (Variables|Default|SetCharacterCreationHelper (Utilities|Array|Get(acopy) _outactors_3)))
                (else
                  (return (Utilities|Array|MakeArray (Transformation|GetActorLocation (Variables|Default|GetCinematicCamera))))))))
          (return (Utilities|Array|MakeArray (Transformation|GetActorLocation _output_get_3) (Transformation|GetActorLocation (Variables|Default|GetCinematicCamera))))))))
  (return (Utilities|Array|MakeArray (Transformation|GetActorLocation _output_get_2))))