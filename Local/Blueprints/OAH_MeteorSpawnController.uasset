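; Meteor spawn controller that runs meteor showers by spawning OAH_MeteorProjectile actors at random points in a box.
; SpawnMeteorShower loops through a randomized count with random delays, aiming meteors from random spawn-box points toward random hit-box points.
; Each valid particle system gets a dynamic material fed the spawner's height for sky fadeout, plus an incrementing translucent sort priority.
; When the shower ends, it resets the cooldown, trigger chance and spawned count.
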(event EventSpawnMeteorShower
  (bind _box (Variables|Default|GetBox))
  (bind _meteorshowerrandomamount (Variables|Default|GetMeteorShowerRandomAmount))
  (bind _returnvalue (Class|FuncomGenericLibrary|GetRandomPointinBox _box))
  (bind _output_get (Variables|Default|SetMeteorShowerTempMaxCount (+ (Variables|Default|GetMeteorShowerMaxCount) (Math|Random|RandomIntegerinRange (* _meteorshowerrandomamount -1) _meteorshowerrandomamount))))
  (if (> _output_get (Variables|Default|GetMeteorShowerAmountSpawned)) :!label _label
    (bind _returnvalue_2 (Game|SpawnActorfromClass "/Game/Mods/OrcsAndHumans/Blueprints/OAH_MeteorProjectile.OAH_MeteorProjectile_C" (Math|Transform|MakeTransform _returnvalue (Math|Rotator|FindLookatRotation _returnvalue (Class|FuncomGenericLibrary|GetRandomPointinBox (Variables|Default|GetHitBox))) "1.000000,1.000000,1.000000") "AlwaysSpawn" self (Math|Vector|MakeVector 0.0 0.0 0.0) 0))
    (Utilities|FlowControl|Delay (Math|Random|RandomFloatinRange 0.05 1.0))
    (Math|Integer|IncrementInt (Variables|Default|GetMeteorShowerAmountSpawned)
      (:%20%20
        (Utilities|IsValid (Variables|/Game/Systems/SkySpawning/BP_MeteorProjectile.BP_MeteorProjectile_C|GetParticleSystem _returnvalue_2)
          (:Is%20Valid
            ;[1 1 1] Give Height information about spawner to material to do fadeout into sky
            (bind _returnvalue_3 (Rendering|Material|CreateDynamicMaterialInstance (Variables|/Game/Systems/SkySpawning/BP_MeteorProjectile.BP_MeteorProjectile_C|GetParticleSystem _returnvalue_2) 0 (Rendering|Material|GetMaterial (Variables|/Game/Systems/SkySpawning/BP_MeteorProjectile.BP_MeteorProjectile_C|GetParticleSystem _returnvalue_2) 0) :!class /Script/Engine.PrimitiveComponent))
            (Rendering|Material|SetScalarParameterValue _returnvalue_3 "spawn_height" (.z (Transformation|GetActorLocation self)) :!class /Script/Engine.MaterialInstanceDynamic)
            (Rendering|SetTranslucentSortPriority (Variables|/Game/Systems/SkySpawning/BP_MeteorProjectile.BP_MeteorProjectile_C|GetParticleSystem _returnvalue_2) (Variables|Default|GetMeteorShowerAmountSpawned))
            (goto _label))
          (:Is%20Not%20Valid
            (goto _label)))))
    (else
      (Variables|Default|SetMeteorCooldown 5)
      (Variables|Default|SetChanceToTriggerMeteor 0)
      (Variables|Default|SetMeteorShowerAmountSpawned 0))))

(fn ConstructionScript
  (|CallParentFunction))